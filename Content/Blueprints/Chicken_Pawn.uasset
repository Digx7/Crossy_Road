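; Player chicken pawn that hops a fixed distance forward, left or right across a world with cars and walls.
; Input sets start and end transforms, then Tick lerps the swept actor and mesh rotation over a timed hop, snaps to the target and fires OnHop.
; Collider hits send the hop back to its start on Wall tags, or play a splat death on Car tags, which stops hop movement.
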(event `InputAction|HopForward`
  (params (Key :type "Key Structure"))
  (:`Pressed`
    (`self.Start_Hop` (1.0 0.0 0.0))))

(event `InputAction|HopLeft`
  (params (Key :type "Key Structure"))
  (:`Pressed`
    (`self.Start_Hop` (0.0 -1.0 0.0))))

(event `InputAction|HopRight`
  (params (Key :type "Key Structure"))
  (:`Pressed`
    (`self.Start_Hop` (0.0 1.0 0.0))))

(event `self.Collider.OnComponentHit`
  (params (HitComponent :type "PrimitiveComponent Object Reference") (OtherActor :type "Actor Object Reference") (OtherComp :type "PrimitiveComponent Object Reference") (NormalImpulse :type "Vector Structure") (Hit :type "HitResult Structure (by ref)"))
  (bind _result (`self.Process_Wall` OtherActor OtherComp))
  (if (not _result)
    (`self.Process_Death` (stale `self.ReceiveActorBeginOverlap` OtherActor))))

(event `self.ReceiveActorBeginOverlap`
  (params (OtherActor :type "Actor Object Reference")))

(event `self.ReceiveTick`
  (params (DeltaSeconds :type "Float (single-precision)"))
  (bind _end_location (`KismetMathLibrary.BreakTransform` (`self.End`)))
  (`|ExecutionSequence`
    (:`then_0`
      (if (`self.Is_Hopping`)
        (if (not (`self.Is Dead`))
          (`self.Process_Hop` DeltaSeconds))))
    (:`then_1`
      (`KismetSystemLibrary.PrintString` (`KismetStringLibrary.Conv_VectorToString` (`self.K2_GetActorLocation`)) true true (struct :`R` 0.047914 :`G` 0.158916 :`B` 1.0 :`A` 1.0) 2.0 "Player"))
    (:`then_2`
      (`KismetSystemLibrary.PrintString` (`KismetStringLibrary.Conv_VectorToString` _end_location) true true (struct :`G` 1.0 :`B` 0.314177 :`A` 1.0) 2.0 "Var"))))

(event `On Hop`
  (params (`Current Location` :type "Vector Structure")))

(fn `Process_Death`
  (params (Other_Actor :type "Actor Object Reference"))
  (if (not (`self.Is Dead`))
    (for _array_element (`Actor.Tags` Other_Actor)
      (switch `name` _array_element
        (:`Car`
          (`KismetSystemLibrary.PrintString` "Your Road Kill!!!" true true (struct :`R` 1.0 :`B` 0.130547 :`A` 1.0))
          (`SkeletalMeshComponent.PlayAnimation` (`self.Chicken_SKM`) "/Game/Animations/Chicken_Death_Splat_Anim.Chicken_Death_Splat_Anim" false)
          (set `self.Is Dead` true))))))

(fn `Process_Hop`
  (params (Delta_Seconds :type "Float (double-precision)"))
  (locals (Mesh_Jump_Start :type "Vector Structure" :default (0.0 0.0 100.0)) (Mesh_Jump_Apex :type "Vector Structure" :default (0.0 0.0 200.0)))
  (bind _end_location (`KismetMathLibrary.BreakTransform` (`self.End`)))
  (bind _max_time (`self.Max Time`))
  (bind _start_location (`KismetMathLibrary.BreakTransform` (`self.Start`)))
  (bind _end_location_2 (`KismetMathLibrary.BreakTransform` (`self.End`)))
  (bind (_start_location_2 _start_rotation) (`KismetMathLibrary.BreakTransform` (`self.Start`)))
  (bind (_end_location_3 _end_rotation) (`KismetMathLibrary.BreakTransform` (`self.End`)))
  (`|ExecutionSequence`
    (:`then_0`
      ;[1 1 1] Times Movement
      (bind _output_get (set `self.Passed Time` (+ Delta_Seconds (`self.Passed Time`))))
      (if (> _output_get (`self.Delay Time`))
        ;[1 1 1] Stops movement
        (if (>= _output_get _max_time)
          (set `self.Passed Time` 0.0)
          (set `self.Is_Hopping` false)
          (`self.K2_SetActorLocation` _end_location false true) ; Snaps the actor to the end position to avoid float-point error bugs
          (`self.OnHop` _end_location)
          (return))))
    (:`then_1`
      (if true
        ;[1 1 1] Rotats Chicken_SKM
        (`SceneComponent.K2_SetRelativeRotation` (`self.Chicken_SKM`) (`KismetMathLibrary.RLerp` _start_rotation _end_rotation (`KismetMathLibrary.NormalizeToRange` _output_get 0.0 _max_time) true) false false)
        ;[1 1 1] Lerps Pawn
        (`self.K2_SetActorLocation` (`KismetMathLibrary.VLerp` _start_location _end_location_2 (`KismetMathLibrary.NormalizeToRange` _output_get 0.0 _max_time)) true)))))

(fn `Process_Wall`
  (params (`Other Actor` :type "Actor Object Reference") (`Other Component` :type "ActorComponent Object Reference"))
  (returns (Result :type Boolean))
  (bind _returnvalue (or (`self.ActorHasTag` `Other Actor` "Wall") (`ActorComponent.ComponentHasTag` `Other Component` "Wall")))
  (if _returnvalue
    (set `self.End` (`self.Start`))
    (set `self.Start` (`KismetMathLibrary.MakeTransform` (`self.K2_GetActorLocation`) (`self.K2_GetActorRotation`)))
    (else
      (return _returnvalue))))

(fn `SetUpCamera`
  (`PlayerController.SetViewTargetWithBlend` (`GameplayStatics.GetPlayerController` 0) (`self.Camera`) 0.0 "VTBlend_Linear" 0.0 false))

(fn `Start_Hop`
  (params (Directon :type "Vector Structure"))
  (bind _returnvalue (`self.K2_GetActorLocation`))
  (bind (_x _y) (`KismetMathLibrary.BreakVector3f` Directon))
  (if (not (`self.Is_Hopping`))
    (set `self.Is_Hopping` true)
    (set `self.Start` (`KismetMathLibrary.MakeTransform` _returnvalue (`SceneComponent.RelativeRotation` (`self.Chicken_SKM`))))
    (set `self.End` (`KismetMathLibrary.MakeTransform` (+ _returnvalue (* Directon (`self.Hop_Distance`))) (`KismetMathLibrary.MakeRotator` 0.0 0.0 (`KismetMathLibrary.DegAtan2` (* _x -1.0) _y))))
    (`SkeletalMeshComponent.PlayAnimation` (`self.Chicken_SKM`) "/Game/Animations/Chicken_Jump_Anim.Chicken_Jump_Anim" false)))

(fn `UserConstructionScript`)