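; Lane is an actor Blueprint for a stretch of floor in a chicken road-crossing game, with a randomized look and detection of the player crossing it.
; Its construction script calls Generate, which applies a random entry from FloorMaterials to the Floor, so the material can reroll whenever construction reruns.
; Actor overlaps go to ChickenDetected, which only prints a crossing message for actors tagged Player.
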(event `self.ReceiveBeginPlay`)

(event `self.ReceiveActorBeginOverlap`
  (params (OtherActor :type "Actor Object Reference"))
  (`self.Chicken_Detected` OtherActor))

(fn `Chicken_Detected`
  (params (`Other Actor` :type "Actor Object Reference"))
  (if (`self.ActorHasTag` `Other Actor` "Player")
    (`KismetSystemLibrary.PrintString` "The Chicken Crossed the Road" true true (struct :`R` 1.0 :`B` 0.862559 :`A` 1.0))))

(fn `Generate`
  (`PrimitiveComponent.SetMaterial` (`self.Floor`) 0 (`KismetArrayLibrary.Array_Random` (`self.FloorMaterials`))))

(fn `UserConstructionScript`
  (`self.Generate`))