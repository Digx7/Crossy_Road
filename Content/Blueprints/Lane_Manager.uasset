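; Lane manager actor that builds a chain of randomly chosen lanes, starting at its own transform when play begins.
; Each spawn picks a random class from LanesToSpawn, registers the manager on the new Lane, and takes that lane's next spawn point as the following spawn transform.
; BeginPlay runs this in a loop to lay down the initial lanes.
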(event `self.ReceiveBeginPlay`
  (`self.Spawn_Initial_Lanes`))

(fn `Spawn_Initial_Lanes`
  (set `self.LaneSpawnTransform` (`self.GetTransform`))
  (for _ (range (+ (`self.InitialAmountOfLanesToSpawn`) 1))
    (`self.Spawn_Lane`)))

(fn `Spawn_Lane`
  (bind _returnvalue (`|SpawnActorFromClass` (`KismetArrayLibrary.Array_Random` (`self.LanesToSpawn`)) (`self.LaneSpawnTransform`) "Undefined" "OverrideRootScale" null null))
  (bind _aslane (cast `/Game/Blueprints/Lane` _returnvalue))
  (bind _output_get (set `self.Latest_Lane` _aslane))
  (`/Game/Blueprints/Lane.Set_Lane_Manager` _output_get self)
  (set `self.LaneSpawnTransform` (`/Game/Blueprints/Lane.NextLaneWorldSpawnPoint` _output_get)))

(fn `UserConstructionScript`)