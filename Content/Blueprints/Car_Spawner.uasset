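; Car spawner actor that repeatedly spawns a randomly chosen class from ObjectsToSpawn at its own transform.
; Tick accumulates delta time until it reaches NextSpawnAt, then resets the timer and rolls the next interval between MinSpawnRate and MaxSpawnRate.
; Despite their names, both rate variables act as delays in seconds between spawns.
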(event `self.ReceiveTick`
  (params (DeltaSeconds :type "Float (single-precision)"))
  (bind _output_get (set `self.Current_Time` (+ DeltaSeconds (`self.Current_Time`))))
  (if (>= _output_get (`self.Next_Spawn_At`))
    (`|ExecutionSequence`
      (:`then_0`
        (set `self.Current_Time` 0.0)
        (set `self.Next_Spawn_At` (`KismetMathLibrary.RandomFloatInRange` (`self.Min_Spawn_Rate`) (`self.Max_Spawn_Rate`))))
      (:`then_1`
        (`|SpawnActorFromClass` (`KismetArrayLibrary.Array_Random` (`self.Objects_To_Spawn`)) (`self.GetTransform`) "Undefined" "OverrideRootScale" null null)))))

(fn `UserConstructionScript`)