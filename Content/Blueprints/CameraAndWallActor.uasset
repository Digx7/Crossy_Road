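; CameraAndWallActor is the player's view target, scrolling steadily along +X and catching up when the Chicken_Pawn hops ahead of it.
; Tick advances a clock and lerps the actor between start and end locations with sweep, starting another constant-speed segment as each finishes.
; The pawn's OnHop event retargets that lerp to the chicken's X over a short catch-up time whenever the chicken lands further forward.
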(event `self.ReceiveBeginPlay`
  (bind _returnvalue (`GameplayStatics.GetActorOfClass` "/Game/Blueprints/Chicken_Pawn.Chicken_Pawn_C"))
  (add `/Game/Blueprints/Chicken_Pawn.OnHop` _returnvalue (delegate `On Hop`))
  (`self.Set Up Camera`)
  (`self.Reset Movement`))

(event `On Hop`
  (params (CurrentLocation :type "Vector Structure"))
  (bind _returnvalue_x (`KismetMathLibrary.BreakVector` (`self.K2_GetActorLocation`)))
  (if (> CurrentLocation_X _returnvalue_x)
    (`self.Update Movement` CurrentLocation_X 0.25)))

(event `self.ReceiveTick`
  (params (DeltaSeconds :type "Float (single-precision)"))
  (bind _passed_time (`self.Clock` DeltaSeconds))
  (`self.Movement` (`self.Start Location`) (`self.End Location`) _passed_time (`self.Max Time`)))

(fn `Clock`
  (params (`Delta Seconds` :type "Float (double-precision)"))
  (returns (`Passed Time` :type "Float (double-precision)"))
  (bind _output_get (set `self.Passed_Time` (+ `Delta Seconds` (`self.Passed_Time`))))
  (return _output_get))

(fn `Movement`
  (params (Start_Location :type "Vector Structure") (End_Location :type "Vector Structure") (PassedTime :type "Float (double-precision)") (MaxTime :type "Float (double-precision)"))
  (bind _returnvalue (`KismetMathLibrary.NormalizeToRange` PassedTime 0.0 MaxTime))
  (if (< _returnvalue 1.0)
    (`self.K2_SetActorLocation` (`KismetMathLibrary.VLerp` Start_Location End_Location _returnvalue) true)
    (else
      (`self.Reset Movement`))))

(fn `Reset Movement`
  (bind _returnvalue_x (`KismetMathLibrary.BreakVector` (`self.K2_GetActorLocation`)))
  (bind _distance (`self.Distance`))
  (`self.Update Movement` (+ _distance _returnvalue_x) (/ _distance 200.0)))

(fn `Set Up Camera`
  (`PlayerController.SetViewTargetWithBlend` (`GameplayStatics.GetPlayerController` 0) self 0.0 "VTBlend_Linear" 0.0 false))

(fn `Update Movement`
  (params (`End Delta X` :type "Float (double-precision)") (`Max Time` :type "Float (double-precision)"))
  (`|ExecutionSequence`
    (:`then_0`
      (bind _output_get (set `self.Start Location` (`self.K2_GetActorLocation`))))
    (:`then_1`
      (set `self.End Location` (`KismetMathLibrary.MakeVector` `End Delta X` (.y _output_get) (.z _output_get))))
    (:`then_2`
      (set `self.Max Time` `Max Time`)
      (set `self.Passed_Time` 0.0))))

(fn `UserConstructionScript`)