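; Road lane actor that randomizes the orientation of its Spawner component, with all other behavior left to its parent class.
; The construction script calls SetUp, which on a random boolean sets the Spawner's relative rotation to a 180-degree turn.
; BeginPlay only forwards to the parent, and the Tick and overlap events are disabled stubs.
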(event `self.ReceiveBeginPlay`
  (`parent.ReceiveBeginPlay`))

(fn `SetUp`
  (if (`KismetMathLibrary.RandomBool`)
    (`SceneComponent.K2_SetRelativeRotation` (`self.Spawner`) (struct :`Yaw` 180.0) false false)))

(fn `UserConstructionScript`
  (`parent.UserConstructionScript`)
  (`self.SetUp`))