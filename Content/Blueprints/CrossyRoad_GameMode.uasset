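; Game mode for a Crossy Road-style game that tracks the game state across start screen, gameplay, kill screen and loading.
; On BeginPlay it binds to the Chicken pawn's hop and death events, so a hop on the start screen begins gameplay and death switches to the kill screen.
; SetCurrentState stores each change and fires a matching event dispatcher per state.
; Tick prints the current state for debugging.
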(event `self.ReceiveBeginPlay`
  (bind _returnvalue (`GameplayStatics.GetActorOfClass` "/Game/Blueprints/Chicken_Pawn.Chicken_Pawn_C"))
  (add `/Game/Blueprints/Chicken_Pawn.OnHop` _returnvalue (delegate `On Hop`))
  (add `/Game/Blueprints/Chicken_Pawn.OnDeath` _returnvalue (delegate `On Death`)))

(event `On Death`
  (`self.Set_CurrentState` "NewEnumerator2"))

(event `On State Update`
  (params (`New State` :type "/Game/Blueprints/Custom_Enums/Game_States Enum" :default "NewEnumerator0")))

(event `On Hop`
  (params (CurrentLocation :type "Vector Structure"))
  (if (`|EnumEquality` (`self.CurrentState`) "NewEnumerator0")
    (`self.Set_CurrentState` "NewEnumerator1")))

(event `self.ReceiveTick`
  (params (DeltaSeconds :type "Float (single-precision)"))
  (`KismetSystemLibrary.PrintString` (`|GetEnumeratorNameAsString` (`self.CurrentState`)) true true (struct :`G` 0.505208 :`B` 0.008877 :`A` 1.0) 2.0 "State"))

(fn `Set_CurrentState`
  (params (NewCurrentState :type "/Game/Blueprints/Custom_Enums/Game_States Enum" :default "NewEnumerator0"))
  (bind _output_get (set `self.CurrentState` NewCurrentState))
  (`self.On State Update` _output_get)
  (switch `/Game/Blueprints/Custom_Enums/Game_States` _output_get
    (:`NewEnumerator0`
      (`self.OnStart_Screen`))
    (:`NewEnumerator1`
      (`self.OnGamePlay`))
    (:`NewEnumerator2`
      (`self.OnKill_Screen`))
    (:`NewEnumerator3`
      (`self.OnLoading`))))

(fn `UserConstructionScript`)